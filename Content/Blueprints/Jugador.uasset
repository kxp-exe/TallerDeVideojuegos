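; Player character Blueprint (Jugador) for a 2D side-scroller, with left/right movement along world X and jumping.
; Axis input feeds AddMovementInput, and the jump action calls Jump and StopJumping.
; Each tick swaps the sprite's flipbook between run and idle based on velocity length.
; It also turns the character by setting controller yaw from the sign of X velocity, keeping the last facing when still.
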(event Custom|Actualizar%20animacion
  (Sprite|SetFlipbook (Variables|Default|GetSprite) (select (> (Math|Vector|VectorLength (Variables|/Script/Engine.MovementComponent|GetVelocity (Variables|Character|GetCharacterMovement))) 0.0) "/Game/Texturas/Main_Characters/Mask_Dude/Run/Run__32x32.Run__32x32" "/Game/Texturas/Main_Characters/Mask_Dude/Idle/Idle__32x32.Idle__32x32")))

(event Custom|Actualizar%20rotacion
  (Math|Float|CompareFloat (.X (Math|Vector|BreakVector (Variables|/Script/Engine.MovementComponent|GetVelocity (Variables|Character|GetCharacterMovement)))) 0.0
    (:>
      (Pawn|SetControlRotation (Pawn|GetController) (Math|Rotator|MakeRotator 0.0 0.0 0.0)))
    (:<
      (Pawn|SetControlRotation (Pawn|GetController) (Math|Rotator|MakeRotator 0.0 0.0 -1.8e+02)))))

(event EventBeginPlay)

(event Collision|EventActorBeginOverlap
  (params (OtherActor :type Actor%20Object%20Reference)))

(event EventTick
  (params (DeltaSeconds :type Float%20%28single-precision%29))
  (CallFunction|ActualizarAnimacion)
  (CallFunction|ActualizarRotacion))

(event Input|ActionEvents|InputActionSaltar
  (params (Key :type Key%20Structure :default "None"))
  (:Pressed
    (Character|Jump))
  (:Released
    (Character|StopJumping)))

(event Input|AxisEvents|InputAxisMoverDerechaIzquierda
  (params (AxisValue :type Float%20%28single-precision%29))
  (Pawn|Input|AddMovementInput "1.000000, 0, 0" AxisValue false))

(fn ConstructionScript)